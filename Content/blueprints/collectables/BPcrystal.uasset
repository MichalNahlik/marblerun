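; Collectable crystal that flies into the player and disappears when the player overlaps it.
; On overlap it stores its starting location, scale and light intensity, then plays a blend timeline.
; Separate timeline tracks lerp it toward the player pawn's live position, shrink it to zero and fade its point light.
; The actor destroys itself when the timeline finishes; no score or inventory change happens here.
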(event Collision|EventActorBeginOverlap
  (params (OtherActor :type Actor%20Object%20Reference))
  (Utilities|ISplayer OtherActor
    (:is%20player
      (CallFunction|StoreStartingValues)
      (bind (_direction _smooth_alpha _scale _light_intensity) (Timeline|Blend%20timeline Play)
        (:Update
          (CallFunction|MovetoPlayer _smooth_alpha)
          (CallFunction|ScaletoPlayer _scale)
          (CallFunction|AdjustLight _light_intensity))
        (:Finished
          (Actor|DestroyActor))))))

(fn ConstructionScript)

(fn MovetoPlayer
  (params (Alpha :type Float%20%28single-precision%29))
  (Transformation|SetActorLocation (Math|Vector|Lerp(Vector) (Variables|Default|GetLerp%20start%20location) (Transformation|GetActorLocation (Game|Player|GetPlayerPawn 0)) Alpha) false false))

(fn StoreStartingValues
  (Variables|Default|SetLerp%20start%20location (Transformation|GetActorLocation))
  (Variables|Default|SetStart%20scale (Transformation|GetActorScale3D))
  (Variables|Default|SetLight%20Intensity (Variables|/Script/Engine.LightComponentBase|GetIntensity (Variables|Default|GetPointLight))))

(fn ScaletoPlayer
  (params (Alpha :type Float%20%28single-precision%29))
  (Transformation|SetActorScale3D (Math|Vector|Lerp(Vector) (Variables|Default|GetStart%20scale) "0, 0, 0" Alpha)))

(fn AdjustLight
  (params (Alpha :type Float%20%28single-precision%29))
  (Rendering|Components|Light|SetIntensity (Variables|Default|GetPointLight) (Math|Float|Lerp (Variables|Default|GetLight%20Intensity) 0.0 Alpha)))