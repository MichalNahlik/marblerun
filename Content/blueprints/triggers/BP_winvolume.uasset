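; BP_winvolume is a trigger volume that completes the level when the player enters it and no crystals remain.
; On overlap, it confirms the actor is the player and checks for any remaining BPcrystal actors in the world.
; Completion finds the current level in the LevelNames array, then opens the next entry by name or quits the game on the last one.
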(event Collision|EventActorBeginOverlap
  (params (OtherActor :type Actor%20Object%20Reference))
  (Utilities|ISplayer OtherActor
    (:is%20player
      (if (not (CallFunction|AnyCrystalsLeft))
        (CallFunction|CompleteLevel)))))

(fn ConstructionScript)

(fn AnyCrystalsLeft
  (bind _outactors (Actor|GetAllActorsOfClass "/Game/blueprints/collectables/BPcrystal.BPcrystal_C"))
  (return (> (Utilities|Array|Length _outactors) 0)))

(fn CompleteLevel
  (if (CallFunction|IsThisFinalLevel)
    (Game|QuitGame 0 "Quit" false)
    (else
      (CallFunction|LoadNextLevel))))

(fn GetCurrentLevelIndex
  (bind _returnvalue (Game|GetCurrentLevelName true))
  (return (Utilities|Array|FindItem (Variables|Default|GetLevel%20names) (Utilities|String|StringToName _returnvalue))))

(fn IsThisFinalLevel
  (return (== (Utilities|Array|LastIndex (Variables|Default|GetLevel%20names)) (CallFunction|GetCurrentLevelIndex))))

(fn LoadNextLevel
  (Game|OpenLevel(byName) (CallFunction|GetNextLevelName)))

(fn GetNextLevelName
  (return (Utilities|Array|Get(acopy) (Variables|Default|GetLevel%20names) (+ (CallFunction|GetCurrentLevelIndex) 1))))