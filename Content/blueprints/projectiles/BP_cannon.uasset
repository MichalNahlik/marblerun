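; BP_cannon is a cannon that automatically fires BP_projectiles on a repeating cycle from BeginPlay.
; After a configurable delay, it spawns a projectile at the spawn point's location and rotation, scaled by ProjectileScale.
; The FireAnimaiton timeline then moves the barrel along its relative Y axis.
; The timeline's Cannon Fired event track loops back to the delay, so no timer or Tick is used.
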(event EventBeginPlay
  (Utilities|FlowControl|Delay (Variables|Default|GetShooting%20delay) :!label _label)
  (CallFunction|SpawnProjectile)
  (bind _fire_movement (Timeline|Fire%20animaiton PlayFromStart)
    (:Update
      (Transformation|SetRelativeLocation (Variables|Default|Getcannon%20barrel) (Math|Vector|MakeVector 0.0 _fire_movement 0.0) false false))
    (:cannon%20fired
      (goto _label))))

(fn ConstructionScript)

(fn SpawnProjectile
  (bind _projectile_spawn_point (Variables|Default|GetProjectile%20spawn%20point))
  (Game|SpawnActorfromClass "/Game/blueprints/projectiles/BP_projectiles.BP_projectiles_C" (Math|Transform|MakeTransform (Transformation|GetWorldLocation _projectile_spawn_point) (Transformation|GetWorldRotation _projectile_spawn_point) (Math|Conversions|ToVector(Float) (Variables|Default|GetProjectile%20scale))) "Undefined" 0 0))